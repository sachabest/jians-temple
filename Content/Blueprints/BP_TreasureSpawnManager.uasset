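; Spawn manager that sets up treasure and Guardian rooms at BeginPlay.
; The server spawns the treasure in a random RoomLocation, then after a short delay yaws every BP_HelpfulStatue toward it.
; It teleports player 0 to an adjacent room index with wraparound, spawning a waterfall, poison pickup and dummy actor there, the dummy serving as the Guardian's target.
; Clients run only the statue rotation, without the delay, using their own TreasureRoomIndex.
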(event `self.ReceiveBeginPlay`
  (bind _returnvalue (`GameplayStatics.GetPlayerCharacter` 0))
  (bind _treasureroom_index (`self.TreasureRoom_Index`))
  (bind _room_location (`self.Room_Location`))
  (bind _item (`KismetArrayLibrary.Array_Get` _room_location (`self.PlayerRoom_Index`)))
  ;[1 1 1] Pick a room and spawn a treasure
  (`/Engine/EditorBlueprintResources/ActorMacros.Switch Has Authority`
    (:`Authority`
      (bind _output_get (set `self.TreasureRoom_Index` (`KismetMathLibrary.RandomInteger` 3)))
      (bind _asactor (castclass `Actor` (`KismetMathLibrary.SelectClass` "/Game/Blueprints/BP_Treasure.BP_Treasure_C" null true)))
      (bind _item_2 (`KismetArrayLibrary.Array_Get` (`self.Room_Location`) _output_get))
      (bind _returnvalue_2 (`|SpawnActorFromClass` _asactor (`KismetMathLibrary.MakeTransform` _item_2) "Undefined" "OverrideRootScale"))
      (bind _asbp_treasure (cast `/Game/Blueprints/BP_Treasure` _returnvalue_2)
        (:`then`
          (set `/Game/Blueprints/BP_Treasure.Chosen_Location` _item_2 _asbp_treasure))
        (:`CastFailed`
          _))
      (`KismetSystemLibrary.Delay` 0.2))
    (:`Remote`
      _))
  ;[1 1 1] Rotate all indicator statues to face treasure room
  (bind _outactors (`GameplayStatics.GetAllActorsOfClass` "/Game/Blueprints/Environment/BP_HelpfulStatue.BP_HelpfulStatue_C"))
  (for _array_element _outactors
    (`self.SetReplicateMovement` _array_element true)
    (`self.SetActorRotation` _array_element (`KismetMathLibrary.MakeRotator` 0.0 0.0 (.yaw (`KismetMathLibrary.Conv_VectorToRotator` (- _item_2 (`self.K2_GetActorLocation` _array_element))))))
    (`/Game/Blueprints/Environment/BP_HelpfulStatue.ClientRotation` _array_element))
  ;[1 1 1] Move Guardian Spawn to an unused treasure room
  (`/Engine/EditorBlueprintResources/ActorMacros.Switch Has Authority`
    (:`Authority`
      (if (<= (`KismetMathLibrary.RandomFloat`) 0.5)
        (bind _output_get_2 (set `self.PlayerRoom_Index` (- _treasureroom_index 1)))
        (if (< _output_get_2 0)
          (set `self.PlayerRoom_Index` (- (`KismetArrayLibrary.Array_Length` _room_location) 1)))
        (else
          (set `self.PlayerRoom_Index` (mod (+ _treasureroom_index 1) (`KismetArrayLibrary.Array_Length` _room_location)))))
      (`|SpawnActorFromClass` "/Game/Blueprints/BP_WaterfallNew.BP_WaterfallNew_C" (`KismetMathLibrary.MakeTransform` (+ _item (0.0 0.0 2000.0))) "Undefined" "OverrideRootScale")
      (`self.K2_SetActorLocation` _returnvalue _item false true)
      ;[1 1 1] Set Return Location for Guardian
      (bind _asbp_guardian (cast `/Game/Characters/BP_Guardian` _returnvalue)
        (:`then`
          (bind _asactor_2 (castclass `Actor` (`KismetMathLibrary.SelectClass` "/Game/Blueprints/BP_Dummy.BP_Dummy_C" null true))
            (:`then`
              (bind _returnvalue_3 (`|SpawnActorFromClass` _asactor_2 (`KismetMathLibrary.MakeTransform` (`KismetMathLibrary.MakeVector` (.x _item) (.y _item) 10.0)) "Undefined" "OverrideRootScale"))
              (set `/Game/Characters/BP_Guardian.TragetActor` _returnvalue_3 _asbp_guardian))
            (:`CastFailed`
              _)))
        (:`CastFailed`
          (`KismetSystemLibrary.PrintString` "Cast To Guardian Failed" true true (struct :`G` 0.66 :`B` 1.0 :`A` 1.0) 20.0)))
      ;[1 1 1] Spawn Poison Pickup Near Guardian
      (bind _asactor_3 (castclass `Actor` (`KismetMathLibrary.SelectClass` "/Game/Blueprints/BP_PickupPoison.BP_PickupPoison_C" null true)))
      (`|SpawnActorFromClass` _asactor_3 (`KismetMathLibrary.MakeTransform` (+ _item (100.0 100.0 -200.0))) "Undefined" "OverrideRootScale"))))

(event `self.ReceiveActorBeginOverlap`
  (params (OtherActor :type "Actor Object Reference")))

(event `self.ReceiveTick`
  (params (DeltaSeconds :type "Float (single-precision)")))

(fn `UserConstructionScript`)