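; Multiplayer game state that ends the match by showing the GameOverWinScreen widget to local player 0 with UI-only input.
; Tick polls for BP_Explorer actors and, with more than one player and none left, shows the screen after a short delay with Win true.
; The ExplorerWin event shows it at once with Win false, and each path runs once.
; The timer OnRep functions are empty.
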(event `self.ReceiveTick`
  (params (DeltaSeconds :type "Float (single-precision)"))
  (if (> (`KismetArrayLibrary.Array_Length` (`self.PlayerArray`)) 1)
    (bind _outactors (`GameplayStatics.GetAllActorsOfClass` "/Game/Characters/BP_Explorer.BP_Explorer_C"))
    (if (== (`KismetArrayLibrary.Array_Length` _outactors) 0)
      (`/Engine/EditorBlueprintResources/StandardMacros.DoOnce` false
        (:`Completed`
          (`KismetSystemLibrary.Delay` 1.0)
          (`/Engine/EditorBlueprintResources/StandardMacros.IsValid` (`self.GameOverScreen`)
            (:`Is Valid`
              _)
            (:`Is Not Valid`
              (bind _returnvalue (`|CreateWidget` "/Game/Blueprints/Widgets/GameOverWinScreen.GameOverWinScreen_C" (`GameplayStatics.GetPlayerController` 0)))
              (bind _output_get (set `self.GameOverScreen` _returnvalue))))
          (`UserWidget.AddToViewport` _output_get 0)
          (`WidgetBlueprintLibrary.SetInputMode_UIOnlyEx` (`GameplayStatics.GetPlayerController` 0) _output_get)
          (set `/Game/Blueprints/Widgets/GameOverWinScreen.Win?` true (`self.GameOverScreen`)))))))

(event `ExplorerWin`
  (`/Engine/EditorBlueprintResources/StandardMacros.DoOnce` false
    (:`Completed`
      (`/Engine/EditorBlueprintResources/StandardMacros.IsValid` (`self.GameOverScreen`)
        (:`Is Valid`
          _)
        (:`Is Not Valid`
          (bind _returnvalue (`|CreateWidget` "/Game/Blueprints/Widgets/GameOverWinScreen.GameOverWinScreen_C" (`GameplayStatics.GetPlayerController` 0)))
          (bind _output_get (set `self.GameOverScreen` _returnvalue))))
      (`UserWidget.AddToViewport` _output_get 0)
      (`WidgetBlueprintLibrary.SetInputMode_UIOnlyEx` (`GameplayStatics.GetPlayerController` 0) _output_get)
      (set `/Game/Blueprints/Widgets/GameOverWinScreen.Win?` false (`self.GameOverScreen`)))))

(fn `OnRep_GameStartTimer`)

(fn `OnRep_RandomTimerValue1`)

(fn `UserConstructionScript`)