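; Thrown torch projectile that immobilizes the first guardian it hits.
; The construction script sets the projectile movement velocity and applies an angular impulse to the collision box.
; A one-shot hit handler splits by network role: authority calls Immobilize on the main guardian, while remote calls ServerImmobilize on any other guardian.
; Both calls pass player controller 0.
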(event `self.ReceiveBeginPlay`)

(event `self.ReceiveActorBeginOverlap`
  (params (OtherActor :type "Actor Object Reference")))

(event `self.ReceiveTick`
  (params (DeltaSeconds :type "Float (single-precision)")))

(event `self.ReceiveHit`
  (params (MyComp :type "PrimitiveComponent Object Reference") (Other :type "Actor Object Reference") (OtherComp :type "PrimitiveComponent Object Reference") (bSelfMoved :type Boolean) (HitLocation :type "Vector Structure") (HitNormal :type "Vector Structure") (NormalImpulse :type "Vector Structure") (Hit :type "HitResult Structure (by ref)"))
  (bind _returnvalue (`GameplayStatics.GetPlayerController` 0))
  ;[1 1 1] Immobilize guardians on hit
  (bind _asbp_guardian (cast `/Game/Characters/BP_Guardian` Other))
  (`/Engine/EditorBlueprintResources/StandardMacros.DoOnce` false
    (:`Completed`
      (`/Engine/EditorBlueprintResources/ActorMacros.Switch Has Authority`
        (:`Authority`
          (bind _ismainguardian (`/Game/Characters/BP_Guardian.IsMainGuardian` _asbp_guardian))
          (if _ismainguardian
            (`/Game/Characters/BP_Guardian.Immobilize` _asbp_guardian _returnvalue)))
        (:`Remote`
          (if (not _ismainguardian)
            (`/Game/Characters/BP_Guardian.ServerImmobilize` _asbp_guardian _returnvalue)))))))

(fn `UserConstructionScript`
  (set `MovementComponent.Velocity` (`self.Initial Velocity`) (`self.ProjectileMovement`))
  (`PrimitiveComponent.AddAngularImpulse` (`self.BoxCollision`) (`self.InitialAngularImpluse`) "None" false))