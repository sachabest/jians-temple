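; Poison projectile that calls HitByPoison on the BP_Explorer it hits.
; The construction script sets the projectile movement velocity from InitialVelocity and applies an angular impulse to its collision box.
; On Hit, separate DoOnce gates limit the poison call to once and spawn the P_Hit emitter once at the hit location, whatever was struck.
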(event `self.ReceiveBeginPlay`)

(event `/Game/Blueprints/Projectiles/BP_ProjectileTorch.ReceiveActorBeginOverlap`
  (params (OtherActor :type "Actor Object Reference")))

(event `self.ReceiveTick`
  (params (DeltaSeconds :type "Float (single-precision)")))

(event `self.ReceiveHit`
  (params (MyComp :type "PrimitiveComponent Object Reference") (Other :type "Actor Object Reference") (OtherComp :type "PrimitiveComponent Object Reference") (bSelfMoved :type Boolean) (HitLocation :type "Vector Structure") (HitNormal :type "Vector Structure") (NormalImpulse :type "Vector Structure") (Hit :type "HitResult Structure (by ref)"))
  ;[1 1 1] Immobilize guardians on hit
  (`|ExecutionSequence`
    (:`then_0`
      (bind _asbp_explorer (cast `/Game/Characters/BP_Explorer` Other))
      (`/Engine/EditorBlueprintResources/StandardMacros.DoOnce` false
        (:`Completed`
          (`/Game/Characters/BP_Explorer.HitByPoison` _asbp_explorer))))
    (:`then_1`
      (`/Engine/EditorBlueprintResources/StandardMacros.DoOnce` false
        (:`Completed`
          (`GameplayStatics.SpawnEmitterAtLocation` "/Game/Effects/P_Hit.P_Hit" HitLocation))))))

(fn `UserConstructionScript`
  (set `MovementComponent.Velocity` (`self.Initial Velocity`) (`self.ProjectileMovement`))
  (`PrimitiveComponent.AddAngularImpulse` (`self.BoxCollision`) (`self.InitialAngularImpluse`) "None" false))