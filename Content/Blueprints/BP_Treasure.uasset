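; Treasure actor that places itself in one of three rooms at random and reacts when an Explorer or Guardian touches it.
; On BeginPlay the server teleports it, moves player 0 (the intended Guardian) to the next room, and spawns a poison pickup there.
; Server-side overlap plays an explosion and sound once per character type, announcing an Explorer's find; the Guardian branch prints only test text.
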(event `self.ReceiveBeginPlay`
  (bind _room_location (`self.Room_Location`))
  ;[1 1 1] Single Treasure will spawn in a random room
  (`/Engine/EditorBlueprintResources/ActorMacros.Switch Has Authority`
    (:`Authority`
      (bind _output_get (set `self.Room Index` (`KismetMathLibrary.RandomInteger` 3)))
      (bind _item (`KismetArrayLibrary.Array_Get` _room_location _output_get))
      (`self.K2_SetActorLocation` _item false true)
      (`SceneComponent.K2_SetWorldLocation` (`self.DefaultSceneRoot`) _item false false)
      (bind _item_2 (`KismetArrayLibrary.Array_Get` _room_location (mod (+ _output_get 1) 3)))
      ;[1 1 1] Spawn the Guardian Elsewhere
      (`self.K2_SetActorLocation` (`GameplayStatics.GetPlayerCharacter` 0) _item_2 false true)
      (bind _asactor (castclass `Actor` (`KismetMathLibrary.SelectClass` "/Game/Blueprints/BP_PickupPoison.BP_PickupPoison_C" null true)))
      (`|SpawnActorFromClass` _asactor (`KismetMathLibrary.MakeTransform` (+ _item_2 (100.0 100.0 -200.0))) "Undefined" "OverrideRootScale"))))

(event `self.ReceiveActorBeginOverlap`
  (params (OtherActor :type "Actor Object Reference"))
  (bind _returnvalue (`self.K2_GetActorLocation`))
  (`/Engine/EditorBlueprintResources/ActorMacros.Switch Has Authority`
    (:`Authority`
      (cast `/Game/Characters/BP_Explorer` OtherActor
        (:`then`
          (`/Engine/EditorBlueprintResources/StandardMacros.DoOnce` false
            (:`Completed`
              (`GameplayStatics.SpawnEmitterAtLocation` "/Game/StarterContent/Particles/P_Explosion.P_Explosion" _returnvalue)
              (`GameplayStatics.PlaySoundAtLocation` "/Game/Sounds/Coin_01.Coin_01" _returnvalue)
              (`KismetSystemLibrary.PrintText` "An Explorer has found the artifact!" true true (struct :`G` 0.66 :`B` 1.0 :`A` 1.0) 4.0))))
        (:`CastFailed`
          (cast `/Game/Characters/BP_Guardian` OtherActor)
          (`/Engine/EditorBlueprintResources/StandardMacros.DoOnce` false
            (:`Completed`
              (`GameplayStatics.SpawnEmitterAtLocation` "/Game/StarterContent/Particles/P_Explosion.P_Explosion" _returnvalue)
              (`GameplayStatics.PlaySoundAtLocation` "/Game/Sounds/Powerup_01.Powerup_01" _returnvalue)
              (`KismetSystemLibrary.PrintText` "TEST"))))))))

(event `self.ReceiveTick`
  (params (DeltaSeconds :type "Float (single-precision)")))

(fn `UserConstructionScript`)