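; BP_DWall is a destructible wall that breaks when a charging BP_Guardian hits it.
; The Hit event casts the other actor to BP_Guardian, checks IsCharging, then passes the hit location and normal to ReplicateDamage.
; That event damages the Destructible with a strong impulse along the normal, spawns destruction and explosion emitters flagged as replicated, and plays an explosion sound at the impact.
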(event `self.ReceiveBeginPlay`)

(event `self.ReceiveActorBeginOverlap`
  (params (OtherActor :type "Actor Object Reference")))

(event `self.ReceiveTick`
  (params (DeltaSeconds :type "Float (single-precision)")))

(event `self.ReceiveHit`
  (params (MyComp :type "PrimitiveComponent Object Reference") (Other :type "Actor Object Reference") (OtherComp :type "PrimitiveComponent Object Reference") (bSelfMoved :type Boolean) (HitLocation :type "Vector Structure") (HitNormal :type "Vector Structure") (NormalImpulse :type "Vector Structure") (Hit :type "HitResult Structure (by ref)"))
  ;[1 1 1] Hit by charging guardian
  (bind _asbp_guardian (cast `/Game/Characters/BP_Guardian` Other))
  (if (`/Game/Characters/BP_Guardian.IsCharging` _asbp_guardian)
    (`self.ReplicateDamage` HitLocation HitNormal)))

(event `ReplicateDamage`
  (params (HitLocation :type "Vector Structure") (HitNormal :type "Vector Structure"))
  ;[1 1 1] Hit by charging guardian
  (`DestructibleComponent.ApplyDamage` (`self.Destructible`) 1.0 HitLocation HitNormal 50000.0)
  (bind _returnvalue (`GameplayStatics.SpawnEmitterAtLocation` "/Game/ExampleContent/Destructibles/Effects/P_Destruction.P_Destruction" HitLocation))
  (`ActorComponent.SetIsReplicated` _returnvalue true)
  (bind _returnvalue_2 (`GameplayStatics.SpawnEmitterAtLocation` "/Game/StarterContent/Particles/P_Explosion.P_Explosion" HitLocation))
  (`ActorComponent.SetIsReplicated` _returnvalue_2 true)
  (`GameplayStatics.PlaySoundAtLocation` "/Game/StarterContent/Audio/Explosion02.Explosion02" HitLocation))

(fn `UserConstructionScript`)