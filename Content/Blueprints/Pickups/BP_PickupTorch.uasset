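; Torch pickup that an explorer collects on overlap, replacing it with a held torch attached to the right-hand grip socket.
; Server-side overlap logic spawns the held torch with the same lit state, or passes fire between the pickup and a torch the explorer already holds.
; A guardian touching an active pickup extinguishes it and gains a charge.
; The replicated IsActive flag drives the Fire component through its RepNotify.
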(event `self.ReceiveBeginPlay`)

(event `self.ReceiveTick`
  (params (DeltaSeconds :type "Float (single-precision)")))

(event `self.ReceiveActorBeginOverlap`
  (params (OtherActor :type "Actor Object Reference"))
  (bind _returnvalue (`ActorComponent.IsActive` (`self.Fire`)))
  ;[1 1 1] Let colliding actor pick me up if the actor is an explorer not holding a torch
  (`/Engine/EditorBlueprintResources/ActorMacros.Switch Has Authority`
    (:`Authority`
      (bind _asbp_explorer (cast `/Game/Characters/BP_Explorer` OtherActor)
        (:`then`
          (bind _throwable (`/Game/Characters/BP_Explorer.Throwable` _asbp_explorer))
          (`/Engine/EditorBlueprintResources/StandardMacros.IsValid` _throwable
            (:`Is Valid`
              (if (`ActorComponent.IsActive` (`/Game/Blueprints/Pickups/BP_TorchHold.Fire` _throwable))
                ;[1 1 1] Lit torch if the colliding explorer is holding a lit torch
                (if (not _returnvalue)
                  (set `self.IsActive` true))
                (else
                  ;[1 1 1] Lit the colliding explorer's torch if it isn't lit and the pick up is lit
                  (if _returnvalue
                    (set `/Game/Blueprints/Pickups/BP_TorchHold.ActivateFire` true _throwable)))))
            (:`Is Not Valid`
              (set `PrimitiveComponent.bGenerateOverlapEvents` false (`self.SphereCollision`))
              (bind _returnvalue_2 (`|SpawnActorFromClass` "/Game/Blueprints/Pickups/BP_TorchHold.BP_TorchHold_C" (`KismetMathLibrary.MakeTransform` (0.0 0.0 0.0)) "AlwaysSpawn" "OverrideRootScale"))
              (set `/Game/Blueprints/Pickups/BP_TorchHold.ActivateFire` (`ActorComponent.IsActive` (`self.Fire`)) _returnvalue_2)
              (`self.K2_AttachRootComponentTo` _returnvalue_2 (`Character.Mesh` _asbp_explorer) "grip_r" "SnapToTarget" true)
              (`self.K2_SetActorRelativeLocation` _returnvalue_2 (0.0 0.0 20.0) false false)
              (set `/Game/Characters/BP_Explorer.Throwable` _returnvalue_2 _asbp_explorer)
              (`self.K2_DestroyActor`))))
        (:`CastFailed`
          ;[1 1 1] Extinguish fire if collide with a guardian
          (bind _asbp_guardian (cast `/Game/Characters/BP_Guardian` OtherActor))
          (if (`self.IsActive`)
            (set `self.IsActive` false)
            (`/Game/Characters/BP_Guardian.IncreaseChargeCount` _asbp_guardian)))))))

(fn `OnRep_IsActive`
  (`ActorComponent.SetActive` (`self.Fire`) (`self.IsActive`) false))

(fn `UserConstructionScript`)