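; PickupBP is a world pickup that a BP_Explorer collects by overlapping it, provided the explorer has no valid Throwable.
; It adds a static mesh component to the explorer, sets it to the pickup's shape and scale, and snaps it to the right grip socket with a small offset.
; The new component becomes the explorer's Throwable, and the pickup actor destroys itself.
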(event `self.ReceiveBeginPlay`)

(event `self.ReceiveActorBeginOverlap`
  (params (OtherActor :type "Actor Object Reference"))
  (bind _asbp_explorer (cast `/Game/Characters/BP_Explorer` OtherActor))
  (`/Engine/EditorBlueprintResources/StandardMacros.IsValid` (`/Game/Characters/BP_Explorer.Throwable` _asbp_explorer)
    (:`Is Not Valid`
      (bind _returnvalue (`AddComponent|Static Mesh Component_856` :`self` _asbp_explorer :`bManualAttachment` true))
      (`StaticMeshComponent.SetStaticMesh` _returnvalue "/Game/Meshes/Pickup_Shape.Pickup_Shape")
      (`SceneComponent.K2_AttachTo` _returnvalue (`Character.Mesh` _asbp_explorer) "grip_r" "SnapToTarget" true)
      (`SceneComponent.SetWorldScale3D` _returnvalue (`SceneComponent.K2_GetComponentScale` (`self.Shape`)))
      (`SceneComponent.K2_SetRelativeLocation` _returnvalue (0.0 0.0 -10.0) false false)
      (set `/Game/Characters/BP_Explorer.Throwable` _returnvalue _asbp_explorer)
      (`self.K2_DestroyActor`))))

(event `self.ReceiveTick`
  (params (DeltaSeconds :type "Float (single-precision)")))

(fn `UserConstructionScript`)