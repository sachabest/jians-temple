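; BP_HelpfulStatue is a statue actor that turns to point toward the treasure's chosen location.
; Its Forcetoturn event takes the first BP_Treasure found in the level and sets the statue's yaw to face that ChosenLocation, zeroing pitch and roll.
; The event disables movement replication before rotating; an authority switch is left unconnected, and nothing in this graph calls the event.
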(event `self.ReceiveBeginPlay`)

(event `self.ReceiveActorBeginOverlap`
  (params (OtherActor :type "Actor Object Reference")))

(event `self.ReceiveTick`
  (params (DeltaSeconds :type "Float (single-precision)")))

(event `Force to turn`
  (bind _outactors (`GameplayStatics.GetAllActorsOfClass` "/Game/Blueprints/BP_Treasure.BP_Treasure_C"))
  (`self.SetReplicateMovement` false)
  (`self.SetActorRotation` (`KismetMathLibrary.MakeRotator` 0.0 0.0 (.yaw (`KismetMathLibrary.Conv_VectorToRotator` (- (`/Game/Blueprints/BP_Treasure.Chosen_Location` (`KismetArrayLibrary.Array_Get` _outactors)) (`self.K2_GetActorLocation`)))))))

(fn `UserConstructionScript`)