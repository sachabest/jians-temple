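; BP_Indicator is a pointer actor that hovers above its owning guardian and aims toward the nearest explorer.
; Each Tick it gathers all BP_Explorer actors, hiding itself when there are none.
; Otherwise FindClosestExplorer picks the nearest by distance to OwnerGuardian, and the actor moves above the guardian with its X axis turned toward that explorer and Z kept upward.
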(event EventBeginPlay)

(event EventActorBeginOverlap
  (params (OtherActor :type Actor%20Object%20Reference)))

(event EventTick
  (params (DeltaSeconds :type Float%20%28single-precision%29))
  (bind _ownerguardian (Variables|Default|GetOwnerGuardian))
  (bind _returnvalue (Transformation|GetActorLocation _ownerguardian))
  (bind _outactors (Actor|GetAllActorsOfClass "/Game/Characters/BP_Explorer.BP_Explorer_C"))
  (if (> (Utilities|Array|Length _outactors) 0)
    (Rendering|SetActorHiddenInGame false)
    (bind _closestexplorer (CallFunction|FindClosestExplorer _outactors))
    (Transformation|SetActorTransform (Math|Transform|MakeTransform (+ _returnvalue "0,0.000000,150.000000") (Math|Rotator|MakeRotfromXZ (- (Transformation|GetActorLocation _closestexplorer) _returnvalue) (Math|Vector|MakeVector 0.0 0.0 1.0)) (Transformation|GetActorScale3D)))
    (else
      (Rendering|SetActorHiddenInGame true))))

(fn ConstructionScript)

(fn FindClosestExplorer
  (params (InExplorers :type Array%20of%20BP%20Explorer%20Object%20References))
  (LocalVariables|SetMinDistance 1e+05)
  (for _array_element InExplorers
    (if (< (Math|Vector|VectorLength (- (Transformation|GetActorLocation _array_element) (Transformation|GetActorLocation (Variables|Default|GetOwnerGuardian)))) (LocalVariables|GetMinDistance))
      (LocalVariables|SetRet _array_element)
      (LocalVariables|SetMinDistance (Math|Vector|VectorLength (- (Transformation|GetActorLocation _array_element) (Transformation|GetActorLocation (Variables|Default|GetOwnerGuardian)))))))
  (return (LocalVariables|GetRet)))