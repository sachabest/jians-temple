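; BP_DestructibleWall is a replicated wall meant to shatter when a charging BP_Guardian hits it.
; BeginPlay stores the static mesh transform for placing the destructible replacement.
; The break logic would consume a charge, swap in a destructible mesh with damage and impulse, then add particles and sound.
; That chain is disconnected from the empty Hit event, so it never runs.
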(event `self.ReceiveBeginPlay`
  ;[1 1 1] Store pos and rot so that we know where to spawn destructible
  (set `self.PosRot` (`SceneComponent.K2_GetComponentToWorld` (`self.StaticMeshComponent`))))

(event `self.ReceiveActorBeginOverlap`
  (params (OtherActor :type "Actor Object Reference")))

(event `self.ReceiveTick`
  (params (DeltaSeconds :type "Float (single-precision)")))

(event `self.ReceiveHit`
  (params (MyComp :type "PrimitiveComponent Object Reference") (Other :type "Actor Object Reference") (OtherComp :type "PrimitiveComponent Object Reference") (bSelfMoved :type Boolean) (HitLocation :type "Vector Structure") (HitNormal :type "Vector Structure") (NormalImpulse :type "Vector Structure") (Hit :type "HitResult Structure (by ref)"))
  ;[1 1 1] Destroy static mesh component. Add destructible mesh component, particle effects, and sound.
)

(fn `UserConstructionScript`
  (`self.SetReplicates` true))