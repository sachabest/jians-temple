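; Static wall actor that randomly decorates both of its sides with BP_PickupTorch actors when play begins.
; On authority only, it compares X and Y scale to find the long axis and derives the torch point count and offsets.
; It steps along evenly spaced points centered on the wall, rolling a small independent chance per side to spawn a torch tilted by a side-specific rotation.
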(event `self.ReceiveBeginPlay`
  (bind _torch_points (`self.Torch_Points`))
  (bind _displacement (`self.Displacement`))
  (bind _x (.x (`self.GetActorScale3D`)))
  (bind _y (.y (`self.GetActorScale3D`)))
  (`/Engine/EditorBlueprintResources/ActorMacros.Switch Has Authority`
    (:`Authority`
      (if (> _x _y)
        ;[1 1 1] Set variables based on X or Y wall orientation
        (set `self.Torch_Points` (- (/ (`KismetMathLibrary.FFloor` _x) 5) 1))
        (set `self.Displacement` (500.0 0.0 0.0))
        (set `self.Rotation Displacement` (20.0 0.0 0.0))
        (set `self.Orthagonal_Displacement` (0.0 75.0 0.0))
        (else
          (set `self.Torch_Points` (- (/ (`KismetMathLibrary.FFloor` _y) 5) 1))
          (set `self.Displacement` (0.0 500.0 0.0))
          (set `self.Rotation Displacement` (0.0 -20.0 0.0))
          (set `self.Orthagonal_Displacement` (75.0 0.0 0.0))))
      ;[1 1 1] Set Initial Spawning Position for Loop Iteration
      (bind _output_get (set `self.Initial_Point` (- (`self.K2_GetActorLocation`) (* _displacement (/ _torch_points 2)))))
      (if (== (mod _torch_points 2) 1)
        (set `self.Initial_Point` (- _output_get (/ _displacement 2.0))))
      ;[1 1 1] For Each Possible Spawning Position
      (for _index (range (+ (`self.Torch_Points`) 1))
        (set `self.Current_Point` (+ (`self.Initial_Point`) (* (`self.Displacement`) _index)))
        (bind _asactor (castclass `Actor` (`KismetMathLibrary.SelectClass` "/Game/Blueprints/Pickups/BP_PickupTorch.BP_PickupTorch_C" null true))
          (:`then`
            ;[1 1 1] Chance to Spawn on One side of wall
            (if (<= (`KismetMathLibrary.RandomFloatInRange` 0.0 1.0) 0.05)
              (`|SpawnActorFromClass` _asactor (`KismetMathLibrary.MakeTransform` (+ (`self.Current_Point`) (`self.Orthagonal_Displacement`)) (`KismetMathLibrary.MakeRotator` (.x (`self.Rotation Displacement`)) (.y (`self.Rotation Displacement`)) (.z (`self.Rotation Displacement`)))) "Undefined" "OverrideRootScale"))
            ;[1 1 1] Chance to Spawn on other side of wall
            (if (<= (`KismetMathLibrary.RandomFloatInRange` 0.0 1.0) 0.05)
              (`|SpawnActorFromClass` _asactor (`KismetMathLibrary.MakeTransform` (- (`self.Current_Point`) (`self.Orthagonal_Displacement`)) (`KismetMathLibrary.MakeRotator` (.x (- (0.0 0.0 0.0) (`self.Rotation Displacement`))) (.y (- (0.0 0.0 0.0) (`self.Rotation Displacement`))) (.z (- (0.0 0.0 0.0) (`self.Rotation Displacement`))))) "Undefined" "OverrideRootScale")))
          (:`CastFailed`
            (`KismetSystemLibrary.PrintString` "Failed to Cast To Actor" true true (struct :`G` 0.66 :`B` 1.0 :`A` 1.0) 5.0)))))))

(event `self.ReceiveActorBeginOverlap`
  (params (OtherActor :type "Actor Object Reference")))

(event `self.ReceiveTick`
  (params (DeltaSeconds :type "Float (single-precision)")))

(fn `UserConstructionScript`)