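; PickupBP is a pickup actor that hands a throwable object to the GuardianBP that overlaps it.
; If that Guardian's Throwable slot is empty, it adds a static mesh component to the Guardian at runtime using Pickup_Shape and the pickup's world scale.
; The component snaps to the grip_r socket with a small offset and is stored as Throwable, then the pickup destroys itself.
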(event `self.ReceiveBeginPlay`)

(event `self.ReceiveActorBeginOverlap`
  (params (OtherActor :type "Actor Object Reference"))
  (bind _asguardian_bp (cast `/Game/Characters/GuardianBP` OtherActor))
  (`/Engine/EditorBlueprintResources/StandardMacros.IsValid` (`/Game/Characters/GuardianBP.Throwable` _asguardian_bp)
    (:`Is Not Valid`
      (bind _returnvalue (`AddComponent|Static Mesh Component_856` :`self` _asguardian_bp :`bManualAttachment` true))
      (`StaticMeshComponent.SetStaticMesh` _returnvalue "/Game/Pickup_Shape.Pickup_Shape")
      (`SceneComponent.K2_AttachTo` _returnvalue (`Character.Mesh` _asguardian_bp) "grip_r" "SnapToTarget" true)
      (`SceneComponent.SetWorldScale3D` _returnvalue (`SceneComponent.K2_GetComponentScale` (`self.Shape`)))
      (`SceneComponent.K2_SetRelativeLocation` _returnvalue (0.0 0.0 -10.0) false false)
      (set `/Game/Characters/GuardianBP.Throwable` _returnvalue _asguardian_bp)
      (`self.K2_DestroyActor`))))

(event `self.ReceiveTick`
  (params (DeltaSeconds :type "Float (single-precision)")))

(fn `UserConstructionScript`)