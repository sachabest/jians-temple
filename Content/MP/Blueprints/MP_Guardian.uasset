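; MP_Guardian is a multiplayer player controller that manages the in-game HUD for its player.
; ClientPostLogin calls SetupGameHUD, which creates W_MP_HUD only for a local controller, stores it as WidgetHUD and adds it to the viewport.
; The login event then casts the game mode to MP_GM with nothing after it, so no spawn logic runs here.
; EndPlay removes the HUD from its parent.
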(event `self.ReceiveBeginPlay`)

(event `ClientPostLogin`
  ;[1 1 1] Setup UI and spawn on login
  (`self.SetupGameHUD`)
  (cast `/Game/MP/Blueprints/MP_GM` (`GameplayStatics.GetGameMode`)))

(event `self.ReceiveTick`
  (params (DeltaSeconds :type "Float (single-precision)")))

(event `self.ReceiveEndPlay`
  (params (EndPlayReason :type "EEndPlayReason Enum" :default "Destroyed"))
  ;[1 1 1] Kill HUD on going back to Main Menu
  (`Widget.RemoveFromParent` (`self.Widget_HUD`)))

(fn `SetupGameHUD`
  (if (`self.IsLocalPlayerController`)
    (bind _returnvalue (`|CreateWidget` "/Game/MP/Widgets/W_MP_HUD.W_MP_HUD_C" self))
    (bind _output_get (set `self.Widget_HUD` _returnvalue))
    (`UserWidget.AddToViewport` _output_get 0)))

(fn `UserConstructionScript`)