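; Multiplayer game mode that handles player login and respawning of MP_Guardian pawns.
; On PostLogin with authority, it sorts PlayerStarts into "Explorer" (Player1) and all others (Player2), then sets PlayerNumber from the player count.
; It then attempts ClientPostLogin through an MP_Guardian cast of the new controller.
; RespawnPlayerEvent replaces the controlled pawn at the first start for that side, treating the first PlayerArray entry as Player1, and possesses it.
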(event `self.ReceiveBeginPlay`)

(event `RespawnPlayerEvent`
  (params (PlayerController :type "PlayerController Object Reference"))
  ;[1 1 1] Spawn Players
  (`self.K2_DestroyActor` (`Controller.K2_GetPawn` PlayerController))
  (if (== (`PlayerState.PlayerId` (`KismetArrayLibrary.Array_Get` (`GameState.PlayerArray` (`GameplayStatics.GetGameState`)))) (`PlayerState.PlayerId` (`Controller.PlayerState` PlayerController)))
    (`|SpawnActorFromClass` "/Game/MP/Blueprints/MP_Guardian.MP_Guardian_C" (`self.GetTransform` (`KismetArrayLibrary.Array_Get` (`self.Player1`))) "AdjustIfPossibleButAlwaysSpawn" "OverrideRootScale")
    (`Controller.Possess` PlayerController null)
    (else
      (`|SpawnActorFromClass` "/Game/MP/Blueprints/MP_Guardian.MP_Guardian_C" (`self.GetTransform` (`KismetArrayLibrary.Array_Get` (`self.Player2`))) "AdjustIfPossibleButAlwaysSpawn" "OverrideRootScale")
      (`Controller.Possess` PlayerController null))))

(event `self.ReceiveTick`
  (params (DeltaSeconds :type "Float (single-precision)")))

(event `self.K2_PostLogin`
  (params (NewPlayer :type "PlayerController Object Reference"))
  ;[1 1 1] Post Login Execution Chain
  (`/Engine/EditorBlueprintResources/ActorMacros.Switch Has Authority`
    (:`Authority`
      (bind _outactors (`GameplayStatics.GetAllActorsOfClass` "/Script/Engine.PlayerStart"))
      (for _array_element _outactors
        (if (== (`PlayerStart.PlayerStartTag` _array_element) "Explorer")
          (`KismetArrayLibrary.Array_AddUnique` (`self.Player1`) _array_element)
          (else
            (`KismetArrayLibrary.Array_AddUnique` (`self.Player2`) _array_element))))
      (bind _asgs_ps (cast `/Game/MP/Blueprints/GS_PS` (`Controller.PlayerState` NewPlayer)))
      ;;[1 1 1] Verifies list in same order
      (set `/Game/MP/Blueprints/GS_PS.PlayerNumber` (`KismetArrayLibrary.Array_Length` (`GameState.PlayerArray` (`GameplayStatics.GetGameState`))) _asgs_ps)
      (bind _asmp_guardian (cast `/Game/MP/Blueprints/MP_Guardian` NewPlayer))
      (`/Game/MP/Blueprints/MP_Guardian.ClientPostLogin` _asmp_guardian))))

(fn `UserConstructionScript`)