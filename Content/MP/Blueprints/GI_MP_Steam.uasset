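; Multiplayer Game Instance (GI_MP_Steam) that manages menus, session hosting and joining, and error reporting.
; A StateTransition macro acts as a finite state machine, cleaning up the current state's widget or session before switching and rejecting same-state requests.
; Menu, server list and loading screen events lazily create their widgets on entering their state.
; Session, network and travel failures route to DisplayError, which destroys the session and handles the error dialog.
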(event `ShowMainMenuEvent`
  (bind _returnvalue (`GameplayStatics.GetPlayerController` 0))
  ;[1 1 1] Show Main Menu
  (`self.StateTransition` "NewEnumerator1"
    (:`SameState`
      (`self.DisplayError` "Couldn't transition to main menu"))
    (:`NewState`
      (`/Engine/EditorBlueprintResources/StandardMacros.IsValid` (`self.MainMenu`)
        (:`Is Valid`
          _)
        (:`Is Not Valid`
          (bind _returnvalue_2 (`|CreateWidget` "/Game/MP/Widgets/W_MainMenu.W_MainMenu_C" _returnvalue))
          (bind _output_get (set `self.MainMenu` _returnvalue_2))))
      (`UserWidget.AddToViewport` _output_get 0)
      (`WidgetBlueprintLibrary.SetInputMode_UIOnlyEx` _returnvalue _output_get))))

(event `HostGameEvent`
  ;[1 1 1] Host Game - called from Main Menu
  (`self.ShowLoadScren`)
  (`CreateSessionCallbackProxy.CreateSession` (`GameplayStatics.GetPlayerController` 0) 4 (`self.bEnableLAN`)
    (:`OnSuccess`
      (`GameplayStatics.OpenLevel` "MP_Level1" true "listen"))
    (:`OnFailure`
      (`self.DisplayError` "Error: Could not create session."))))

(event `DestroySessionEvent`
  ;[1 1 1] Called to end player sessions
  (`DestroySessionCallbackProxy.DestroySession` (`GameplayStatics.GetPlayerController` 0)))

(event `JoinFromServerListEvent`
  (params (SearchResult :type "BlueprintSessionResult Structure"))
  ;[1 1 1] Join a server, show a loading screen, and handle errors
  (`self.ShowLoadScren`)
  (`JoinSessionCallbackProxy.JoinSession` (`GameplayStatics.GetPlayerController` 0) SearchResult
    (:`OnFailure`
      (`self.DisplayError` "Failed to join server!"))))

(event `ShowServerListEvent`
  (bind _returnvalue (`GameplayStatics.GetPlayerController` 0))
  ;[1 1 1] Show server list from Main Menu
  (`self.StateTransition` "NewEnumerator4"
    (:`NewState`
      (`/Engine/EditorBlueprintResources/StandardMacros.IsValid` (`self.ServerList`)
        (:`Is Valid`
          _)
        (:`Is Not Valid`
          (bind _returnvalue_2 (`|CreateWidget` "/Game/MP/Widgets/W_serverList.W_serverList_C" _returnvalue))
          (bind _output_get (set `self.ServerList` _returnvalue_2))))
      (`UserWidget.AddToViewport` _output_get 0)
      (`WidgetBlueprintLibrary.SetInputMode_UIOnlyEx` _returnvalue _returnvalue_2))))

(event `ShowLoadScren`
  (bind _returnvalue (`GameplayStatics.GetPlayerController` 0))
  ;[1 1 1] Show loading screen when changing maps
  (`self.StateTransition` "NewEnumerator6"
    (:`NewState`
      (`/Engine/EditorBlueprintResources/StandardMacros.IsValid` (`self.Loading`)
        (:`Is Valid`
          _)
        (:`Is Not Valid`
          (bind _returnvalue_2 (`|CreateWidget` "/Game/MP/Widgets/W_LoadingScreen.W_LoadingScreen_C" _returnvalue))
          (bind _output_get (set `self.Loading` _returnvalue_2))))
      (`UserWidget.AddToViewport` _output_get 0)
      (`WidgetBlueprintLibrary.SetInputMode_UIOnlyEx` _returnvalue))))

(event `self.HandleNetworkError`
  (params (FailureType :type "ENetworkFailure Enum" :default "NetDriverAlreadyExists") (bIsServer :type Boolean))
  ;[1 1 1] Catch network errors during map transitions
  (if (not bIsServer)
    (`self.DisplayError` (`self.NetCodeErrorToString` FailureType))))

(event `self.HandleTravelError`
  (params (FailureType :type "ETravelFailure Enum" :default "NoLevel"))
  ;[1 1 1] Catch network errors during map transitions
  (`self.DisplayError` (`self.TravelErrorToString` FailureType)))

(fn `BeginPlay_ShowMainMenu`
  ;[1 1 1] Show Main Menu on Game Open
  (`self.StateTransition` "NewEnumerator0"
    (:`SameState`
      (`self.ShowMainMenuEvent`))))

(fn `HideWidget`
  (params (WidgetIn :type "Widget Object Reference"))
  (`Widget.RemoveFromParent` WidgetIn))

(fn `NetCodeErrorToString`
  (params (NetError :type "ENetworkFailure Enum"))
  (returns (ErrorOut :type String))
  (switch `ENetworkFailure` NetError
    (:`NetDriverAlreadyExists`
      _)
    (:`NetDriverCreateFailure`
      _)
    (:`NetDriverListenFailure`
      _)
    (:`ConnectionLost`
      _)
    (:`ConnectionTimeout`
      (return "Error: connection timeout."))
    (:`FailureReceived`
      _)
    (:`OutdatedClient`
      _)
    (:`OutdatedServer`
      _)
    (:`PendingConnectionFailure`
      _))
  (return "Error: lost connection to host."))

(fn `StartPlayingState`
  (`self.StateTransition` "NewEnumerator2"))

(fn `TravelErrorToString`
  (params (TravelError :type "ETravelFailure Enum"))
  (returns (ErrorString :type String))
  (return (`KismetStringLibrary.Concat_StrStr` "Error travelling maps  due to:" (`|GetEnumeratorNameAsString` TravelError))))