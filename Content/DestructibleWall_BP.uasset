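; Destructible wall actor that shatters when a charging Guardian pawn hits it.
; BeginPlay caches the static mesh's world transform for spawning the destructible replacement.
; On the first qualifying Hit, gated by DoOnce, it destroys the static mesh and adds a destructible mesh component at that transform.
; It then applies damage with an impulse along the hit normal and plays destruction and explosion particles plus a sound.
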(event `self.ReceiveBeginPlay`
  ;[1 1 1] Store pos and rot so that we know where to spawn destructible
  (set `self.PosRot` (`SceneComponent.K2_GetComponentToWorld` (`self.StaticMeshComponent`))))

(event `self.ReceiveActorBeginOverlap`
  (params (OtherActor :type "Actor Object Reference")))

(event `self.ReceiveTick`
  (params (DeltaSeconds :type "Float (single-precision)")))

(event `self.ReceiveHit`
  (params (MyComp :type "PrimitiveComponent Object Reference") (Other :type "Actor Object Reference") (OtherComp :type "PrimitiveComponent Object Reference") (bSelfMoved :type Boolean) (HitLocation :type "Vector Structure") (HitNormal :type "Vector Structure") (NormalImpulse :type "Vector Structure") (Hit :type "HitResult Structure (by ref)"))
  (bind _returnvalue (+ HitLocation (0.0 0.0 20.0)))
  ;[1 1 1] Destroy static mesh component. Add destructible mesh component, particle effects, and sound.
  (bind _asguardian_bp (cast `/Game/Characters/GuardianBP` Other))
  (if (`/Game/Characters/GuardianBP.IsCharging` _asguardian_bp)
    (`/Engine/EditorBlueprintResources/StandardMacros.DoOnce` false
      (:`Completed`
        (`ActorComponent.K2_DestroyComponent` (`self.StaticMeshComponent`))
        (bind _returnvalue_2 (`AddComponent|Destructible Component_4` :`RelativeTransform` (`self.PosRot`)))
        (`DestructibleComponent.SetDestructibleMesh` _returnvalue_2 "/Game/Wall_500x500_DM.Wall_500x500_DM")
        (`DestructibleComponent.ApplyDamage` _returnvalue_2 1.0 (- HitLocation (* HitNormal 50.0)) HitNormal 50000.0)
        (bind _returnvalue_3 (`GameplayStatics.SpawnEmitterAtLocation` "/Game/ExampleContent/Destructibles/Effects/P_Destruction.P_Destruction" _returnvalue))
        (`SceneComponent.SetWorldScale3D` _returnvalue_3 (1.0 1.0 1.0))
        (`GameplayStatics.SpawnEmitterAtLocation` "/Game/StarterContent/Particles/P_Explosion.P_Explosion" _returnvalue)
        (`GameplayStatics.PlaySoundAtLocation` "/Game/StarterContent/Audio/Explosion02.Explosion02" HitLocation)))))

(fn `UserConstructionScript`)