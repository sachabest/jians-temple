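; BP_AI_CloseEnough is an AI condition check that reports whether the controlled pawn is within an acceptable distance of its blackboard target location.
; It casts the owner to BP_AI, caches it, then compares the vector distance from that controller's pawn to the TargetLocation key against AcceptableDistance.
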(fn `PerformConditionCheck`
  (params (OwnerActor :type "Actor Object Reference"))
  (returns (ReturnValue :type Boolean))
  (bind _asbp_ai (cast `/Game/AI/BP_AI` OwnerActor)
    (:`then`
      (set `self.AI_CON_Ref` _asbp_ai))
    (:`CastFailed`
      _))
  (return (< (`KismetMathLibrary.VSize` (- (`BTFunctionLibrary.GetBlackboardValueAsVector` (`self.TargetLocation`)) (`Actor.K2_GetActorLocation` (`Controller.K2_GetPawn` (`self.AI_CON_Ref`))))) (`self.AcceptableDistance`))))