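; Behavior tree node for the AI that sets a TargetLocation blackboard vector, apparently the destination for running home.
; Each tick it caches the BP_AI controller, then sphere-traces a wide radius around its pawn for desired object types.
; A Camera-channel line trace checks line of sight to each hit, ignoring all actors of a class.
; Every visible hit overwrites TargetLocation, so the last one wins rather than the nearest.
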(event `self.ReceiveTick`
  (params (OwnerActor :type "Actor Object Reference") (DeltaSeconds :type "Float (single-precision)"))
  (bind _returnvalue (`Actor.K2_GetActorLocation` (`Controller.K2_GetPawn` (`self.AI_CON_Ref`))))
  ;[1 1 1] Is AI_CON_Ref set?
  (if (not (!= (`self.AI_CON_Ref`) null))
    (bind _asbp_ai (cast `/Game/AI/BP_AI` OwnerActor))
    (set `self.AI_CON_Ref` _asbp_ai))
  (bind _outactors (`GameplayStatics.GetAllActorsOfClass` null))
  (set `self.MyLocation` _returnvalue)
  (bind _outhits (`KismetSystemLibrary.SphereTraceMultiForObjects` _returnvalue (+ _returnvalue (0.0 0.0 15.0)) 1500.0 (`self.DesiredObjectTypes`) false _outactors))
  (for _array_element _outhits
    (bind (_bblockinghit _binitialoverlap _time _location _impactpoint _normal _impactnormal _physmat _hitactor) (`GameplayStatics.BreakHitResult` _array_element))
    (bind _outhit (`KismetSystemLibrary.LineTraceSingle` (`self.MyLocation`) (`Actor.K2_GetActorLocation` _hitactor) "TraceTypeQuery2" false _outactors))
    (bind (_bblockinghit_2 _binitialoverlap_2 _time_2 _location_2 _impactpoint_2 _normal_2 _impactnormal_2 _physmat_2 _hitactor_2) (`GameplayStatics.BreakHitResult` _outhit))
    (if (== _hitactor_2 _hitactor)
      (`BTFunctionLibrary.SetBlackboardValueAsVector` (`self.TargetLocation`) (`Actor.K2_GetActorLocation` _hitactor_2)))))